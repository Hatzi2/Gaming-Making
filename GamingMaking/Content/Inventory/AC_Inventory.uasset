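; Inventory actor component that stores items in a slot-keyed map and toggles the UMG_Inventory widget, cursor and input mode on IA_Inventory.
; PickUpItem scans slots up to MaxSize for matching items and the first empty slot, respecting MaxStack and AllowDuplicates.
; Widget events write slot additions and removals back to the map.
; Dropped items spawn as A_Item at a downward box-trace impact point ahead of the owner.
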(event `self.ReceiveBeginPlay`
  (`EnhancedInputSubsystemInterface.AddMappingContext` (pcsubsystem `EnhancedInputLocalPlayerSubsystem` (`GameplayStatics.GetPlayerController` 0)) "/Game/Inventory/IMC_Inventory.IMC_Inventory" 0 (struct)))

(event `EnhancedInput|/Game/Inventory/IA_Inventory`
  (params (ActionValue :type Boolean) (ElapsedSeconds :type "Float (double-precision)") (TriggeredSeconds :type "Float (double-precision)") (InputAction :type "InputAction Object Reference" :default "/Game/Inventory/IA_Inventory.IA_Inventory"))
  (bind _returnvalue (`GameplayStatics.GetPlayerController` 0))
  (bind _returnvalue_2 (`GameplayStatics.GetPlayerController` 0))
  (bind _as_umg_inventory (`self.AS UMG_Inventory`))
  (:`Started`
    (`self.AS UMG_Inventory`
      (:`then`
        (set `PlayerController.bShowMouseCursor` false _returnvalue)
        (`WidgetBlueprintLibrary.SetInputMode_GameOnly` _returnvalue true)
        (`Widget.RemoveFromParent` (`self.AS UMG_Inventory`))
        (set `self.AS UMG_Inventory` null))
      (:`else`
        (bind _returnvalue_3 (`|CreateWidget` "/Game/Inventory/Widgets/UMG_Inventory.UMG_Inventory_C" null (`self.Inventory`) (`self.MaxSize`) (`self.AllowDuplicates`) self))
        (bind _output_get (set `self.AS UMG_Inventory` _returnvalue_3))
        (`UserWidget.AddToViewport` _output_get 0)
        (add `/Game/Inventory/Widgets/UMG_Inventory.ItemAdded` _as_umg_inventory (`|CreateDelegate` :!event `ItemAdded`))
        (add `/Game/Inventory/Widgets/UMG_Inventory.ItemDropped` _as_umg_inventory (`|CreateDelegate` :!event `ItemDropped`))
        (add `/Game/Inventory/Widgets/UMG_Inventory.ItemRemoved` _as_umg_inventory (`|CreateDelegate` :!event `ItemRemoved`))
        (set `PlayerController.bShowMouseCursor` true _returnvalue_2)
        (`WidgetBlueprintLibrary.SetInputMode_GameAndUIEx` _returnvalue_2 null)))))

(fn `IsKeyFull`
  (params (Key :type Integer))
  (returns (ReturnValue :type Boolean) (Remaining :type Integer))
  (bind (_value _returnvalue) (`BlueprintMapLibrary.Map_Find` (`self.Inventory`) (`local.Key`)))
  (bind (_quantity _dataasset) (break `/Game/Inventory/Items/ST_Inventory` _value))
  (bind _maxstack (`/Game/Inventory/Items/DA_Items.MaxStack` _dataasset))
  (bind _returnvalue_2 (- _maxstack _quantity))
  (if _returnvalue
    (return (and (== _returnvalue_2 0) (!= _maxstack 0)) _returnvalue_2)
    (else
      (return false -1))))

(fn `ItemAdded`
  (params (`Slot key` :type Integer) (`Slot Value` :type "/Game/Inventory/Items/ST_Inventory Structure"))
  (`BlueprintMapLibrary.Map_Add` (`self.Inventory`) `Slot key` `Slot Value`))

(fn `ItemDropped`
  (params (ItemDropped :type "/Game/Inventory/Items/ST_Inventory Structure"))
  (bind _returnvalue (`self.GetOwner`))
  (bind _returnvalue_2 (+ (* (`Actor.GetActorForwardVector` _returnvalue) 300.0) (`Actor.K2_GetActorLocation` _returnvalue)))
  (bind _outhit (`KismetSystemLibrary.BoxTraceSingle` _returnvalue_2 (- _returnvalue_2 (0.0 0.0 500.0)) (15.0 15.0 15.0) (struct) "TraceTypeQuery1" false (`|MakeArray` (`self.GetOwner`))))
  (if true
    (`|SpawnActorFromClass` "/Game/Inventory/Items/A_Item.A_Item_C" (`KismetMathLibrary.MakeTransform` (`.ImpactPoint` (`GameplayStatics.BreakHitResult` _outhit))) "Undefined" "MultiplyWithRoot" null (`local.ItemDropped`) null)))

(fn `ItemRemoved`
  (params (Key :type Integer))
  (`BlueprintMapLibrary.Map_Remove` (`self.Inventory`) Key))

(fn `PickUpItem`
  (params (Item :type "/Game/Inventory/Items/A_Item Object Reference"))
  (returns (ReturnValue :type Boolean))
  (locals (L_QuantityIn :type Integer) (L_DataAssetsIn :type "/Game/Inventory/Items/DA_Items Object Reference") (L_Index :type Integer) (L_FoundSameItem :type Boolean) (L_remaining :type Integer :default 0) (L_EmptyKey :type Integer :default -1))
  (bind (_quantity _dataasset) (break `/Game/Inventory/Items/ST_Inventory` (`/Game/Inventory/Items/A_Item.Structure` Item)))
  (bind (_returnvalue _remaining) (`self.IsKeyFull` (`local.L_Index`)))
  (bind _value (`BlueprintMapLibrary.Map_Find` (`self.Inventory`) (`local.L_Index`)))
  (bind _returnvalue_2 (- (`local.L_QuantityIn`) (`local.L_remaining`)))
  (set `local.L_QuantityIn` _quantity)
  (set `local.L_DataAssetsIn` _dataasset)
  (while (and (> (`local.L_QuantityIn`) 0) (< (`local.L_Index`) (`self.MaxSize`)))
    (`|ExecutionSequence`
      (:`then_0`
        (if _returnvalue
          (if (== (`.DataAsset_5_7B0EC951429F63E6ACE13DA972C4F8A8` (break `/Game/Inventory/Items/ST_Inventory` (`BlueprintMapLibrary.Map_Find` (`self.Inventory`) (`local.L_Index`)))) (`local.L_DataAssetsIn`))
            (set `local.L_FoundSameItem` true))
          (else
            (bind _output_get (set `local.L_remaining` _remaining))
            (if (== _output_get -1)
              (if (== -1 (`local.L_EmptyKey`))
                (set `local.L_EmptyKey` (`local.L_Index`))
                (elif (== (`.DataAsset_5_7B0EC951429F63E6ACE13DA972C4F8A8` (break `/Game/Inventory/Items/ST_Inventory` _value)) (`local.L_DataAssetsIn`))
                  (`BlueprintMapLibrary.Map_Add` (`self.Inventory`) (`local.L_Index`) (make `/Game/Inventory/Items/ST_Inventory` (+ (break `/Game/Inventory/Items/ST_Inventory` _value) (`KismetMathLibrary.Clamp` (`local.L_QuantityIn`) 0 (`local.L_remaining`))) (`local.L_DataAssetsIn`)))
                  (set `local.L_QuantityIn` (`KismetMathLibrary.Clamp` _returnvalue_2 0 _returnvalue_2))
                  (set `local.L_FoundSameItem` true)))))))
      (:`then_1`
        (`/Engine/EditorBlueprintResources/StandardMacros.IncrementInt` (`local.L_Index`)))))
  (if (== (`local.L_QuantityIn`) 0)
    (return true)
    (elif (and (not (`self.AllowDuplicates`)) (`local.L_FoundSameItem`))
      (`/Game/Inventory/Items/A_Item.ModifyQuantity` (`local.Item`) (`local.L_QuantityIn`))
      (return false)
      (elif (!= (`local.L_EmptyKey`) -1)
        (`BlueprintMapLibrary.Map_Add` (`self.Inventory`) (`local.L_EmptyKey`) (make `/Game/Inventory/Items/ST_Inventory` (`local.L_QuantityIn`) (`local.L_DataAssetsIn`)))
        (return true)
        (else
          (return false))))))