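; Animated medieval water wheel prop that drives the moving mesh parts of its mechanism.
; Tick spins two parts continuously at their own speed variables, on pitch and roll respectively, and keeps the first of four chained timelines playing.
; Each timeline's Update starts the next and each restarts on finish, driving one part's roll, another's height, another's roll and another's Z scale.
; A Direction flag flips the sign of both timeline rolls and the scale.
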(event `self.ReceiveBeginPlay`)

(event `self.ReceiveTick`
  (params (DeltaSeconds :type "Float (single-precision)"))
  (`SceneComponent.K2_AddLocalRotation` (`self.SM_water_wheel_part_01`) (* (`KismetMathLibrary.MakeRotator` 0.0 (`self.rotator_speed_01`)) DeltaSeconds) false false)
  (`SceneComponent.K2_AddLocalRotation` (`self.SM_water_wheel_part_02`) (* (`KismetMathLibrary.MakeRotator` (`self.rotator_speed_02`)) DeltaSeconds) false false)
  (bind (_direction _up) (`Timeline|Timeline_0` :!label _label)
    (:`Update`
      (`SceneComponent.K2_SetRelativeRotation` (`self.SM_water_wheel_part_03`) (`KismetMathLibrary.MakeRotator` (* _up (`self.Angle`) (`KismetMathLibrary.SelectFloat` -1.0 1.0 (`self.Direction`)))) false false)
      (bind (_direction_2 _up_2) (`Timeline|Timeline_1` :!label _label_2)
        (:`Update`
          (`SceneComponent.K2_SetRelativeLocation` (`self.SM_water_wheel_part_04`) (`KismetMathLibrary.MakeVector` 140.0 -352.5 _up_2) false false)
          (bind (_direction_3 _up_3) (`Timeline|Timeline_2` :!label _label_3)
            (:`Update`
              (`SceneComponent.K2_SetRelativeRotation` (`self.SM_water_wheel_part_06`) (`KismetMathLibrary.MakeRotator` (* _up_3 (`self.angle_02`) (`KismetMathLibrary.SelectFloat` -1.0 1.0 (`self.Direction`)))) false false)
              (bind (_direction_4 _up_4) (`Timeline|Timeline_3` :!label _label_4)
                (:`Update`
                  (`SceneComponent.SetRelativeScale3D` (`self.SM_water_wheel_part_07`) (`KismetMathLibrary.MakeVector` 1.0 1.0 (* _up_4 (`self.Z`) (`KismetMathLibrary.SelectFloat` -1.0 1.0 (`self.Direction`))))))
                (:`Finished`
                  (goto _label_4 :!via `PlayFromStart`))))
            (:`Finished`
              (goto _label_3 :!via `PlayFromStart`))))
        (:`Finished`
          (goto _label_2 :!via `PlayFromStart`))))
    (:`Finished`
      (goto _label :!via `PlayFromStart`))))

(fn `UserConstructionScript`)