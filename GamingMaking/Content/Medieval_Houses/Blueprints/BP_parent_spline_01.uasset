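; Parent Blueprint for Medieval Houses spline pieces, laying a repeated static mesh along a spline in the construction script.
; Each section gets a spline mesh component with configurable collision, using positions and tangents sampled by distance, with tangents clamped to section length.
; FullLenght keeps only whole sections; otherwise one extra section covers the remainder.
; AllowScaling writes SectionLenght from actor X scale, while placement reads the differently spelled SectionLength.
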(fn `End Position Tangent`
  (params (index :type Integer))
  (returns (position :type "Vector Structure") (tangent :type "Vector Structure"))
  (bind _returnvalue (* (+ index 1) (`self.section length`)))
  (return (`SplineComponent.GetLocationAtDistanceAlongSpline` (`self.Spline`) _returnvalue "Local") (`KismetMathLibrary.ClampVectorSize` (`SplineComponent.GetTangentAtDistanceAlongSpline` (`self.Spline`) _returnvalue "Local") 0.0 (`self.section length`))))

(fn `Start Position Tangent`
  (params (index :type Integer))
  (returns (position :type "Vector Structure") (tangent :type "Vector Structure"))
  (bind _returnvalue (* index (`self.section length`)))
  (return (`SplineComponent.GetLocationAtDistanceAlongSpline` (`self.Spline`) _returnvalue "Local") (`KismetMathLibrary.ClampVectorSize` (`SplineComponent.GetTangentAtDistanceAlongSpline` (`self.Spline`) _returnvalue "Local") 0.0 (`self.section length`))))

(fn `UserConstructionScript`
  (locals (section_lenght :type "Float (double-precision)") (`loop index` :type Integer))
  (bind _returnvalue_x (`KismetMathLibrary.BreakVector` (`self.GetActorScale3D`)))
  (if (`self.allow scaling?`)
    (set `local.section_lenght` (* _returnvalue_x 100.0)))
  (if (`self.full lenght?`)
    (for _index (range (`KismetMathLibrary.FTrunc` (/ (`SplineComponent.GetSplineLength` (`self.Spline`)) (`self.section length`))))
      (set `local.loop index` _index)
      (bind _returnvalue (`AddComponent|NODE_AddSplineMeshComponent-0` :!label _label))
      (`StaticMeshComponent.SetStaticMesh` _returnvalue (`self.spline mesh`))
      (`SplineMeshComponent.SetForwardAxis` _returnvalue "X" true)
      (bind (_position _tangent) (`self.Start Position Tangent` (`local.loop index`)))
      (bind (_position_2 _tangent_2) (`self.End Position Tangent` (`local.loop index`)))
      (`SplineMeshComponent.SetStartAndEnd` _returnvalue _position _tangent _position_2 _tangent_2 true)
      (`PrimitiveComponent.SetCollisionEnabled` _returnvalue (`self.collison type`)))
    (else
      (for _index_2 (range (+ (`KismetMathLibrary.FTrunc` (/ (`SplineComponent.GetSplineLength` (`self.Spline`)) (`self.section length`))) 1))
        (set `local.loop index` _index_2)
        (goto _label)))))